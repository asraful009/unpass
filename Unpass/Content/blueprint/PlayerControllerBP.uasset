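; Player controller that drives the controlled pawn as an auto-runner, constantly moving it forward with player-controlled strafing and look.
; BeginPlay gets the character reference through a pawn message call and sets its walk speed from Speed.
; Tick adds yaw-relative forward input, so the MoveFwd axis does nothing; MoveLeftRight strafes, while Turn and LookUp feed yaw and pitch.
; A getter exposes the controller itself.
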(event EventTick
  (params (DeltaSeconds :type Float%20%28single-precision%29))
  (bind _returnvalue (Pawn|GetControlledPawn))
  (Utilities|IsValid _returnvalue
    (:Is%20Valid
      (Pawn|Input|AddMovementInput _returnvalue (Math|Vector|GetForwardVector (Math|Rotator|MakeRotator 0.0 0.0 (.yaw (Transformation|GetActorRotation _returnvalue)))) 1.0 false))))

(event EventBeginPlay
  (bind _playercharactorref (Class|IFPlayerCharactorBP|GetPlayerCharactorRef(Message) (Game|Player|GetPlayerPawn 0)))
  (Variables|Default|SetPlayerCharactorRef _playercharactorref)
  (Variables|/Script/Engine.CharacterMovementComponent|SetMaxWalkSpeed (Variables|/Script/Engine.Character|GetCharacterMovement (Variables|Default|GetPlayerCharactorRef)) (Variables|Default|GetSpeed)))

(event Input|AxisEvents|InputAxisMoveFwd
  (params (AxisValue :type Float%20%28single-precision%29)))

(event Input|AxisEvents|InputAxisMoveLeftRight
  (params (AxisValue :type Float%20%28single-precision%29))
  (bind _returnvalue (Pawn|GetControlledPawn))
  (Utilities|IsValid _returnvalue
    (:Is%20Valid
      (Pawn|Input|AddMovementInput _returnvalue (Math|Vector|GetRightVector (Math|Rotator|MakeRotator 0.0 0.0 (.yaw (Transformation|GetActorRotation _returnvalue)))) AxisValue false))))

(event Input|AxisEvents|InputAxisTurn
  (params (AxisValue :type Float%20%28single-precision%29))
  (Class|PlayerController|AddYawInput AxisValue))

(event Input|AxisEvents|InputAxisLookUp
  (params (AxisValue :type Float%20%28single-precision%29))
  (Class|PlayerController|AddPitchInput AxisValue))

(fn ConstructionScript)

(fn GetPlayerControllerrEF
  (return self))