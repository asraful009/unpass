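; Player pawn Blueprint that flies with a FloatingPawnMovement component and restarts the level on death.
; Every Tick raises the movement component's max speed at a constant rate toward a fixed cap, regardless of input.
; Forward and sideways inputs add movement along vectors built from control pitch only, with yaw and roll zeroed.
; OnDead prints a message and runs the RestartLevel console command.
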(event Custom|MoveFrd
  (params (intensity :type Float%20%28single-precision%29))
  ;[1 1 1] movementByInput
  (Pawn|Input|AddMovementInput (Math|Vector|GetForwardVector (Math|Rotator|MakeRotator 0.0 (.pitch (Pawn|GetControlRotation :!class /Script/Engine.Pawn)) 0.0)) intensity false))

(event Custom|MoveLeftRight
  (params (influence :type Float%20%28single-precision%29))
  ;[1 1 1] movementByInput
  (Pawn|Input|AddMovementInput (Math|Vector|GetRightVector (Math|Rotator|MakeRotator 0.0 (.pitch (Pawn|GetControlRotation :!class /Script/Engine.Pawn)) 0.0)) influence false))

(event Custom|OnDead
  (Development|PrintString "RestartLevel")
  (Development|ExecuteConsoleCommand "RestartLevel" 0))

(event EventBeginPlay)

(event Collision|EventActorBeginOverlap
  (params (OtherActor :type Actor%20Object%20Reference)))

(event EventTick
  (params (DeltaSeconds :type Float%20%28single-precision%29))
  (bind _output_get (Variables|Default|SetFwdMove (Math|Interpolation|FInterptoConstant (Variables|Default|GetFwdMove) 4e+03 DeltaSeconds 5e+02)))
  (Variables|/Script/Engine.FloatingPawnMovement|SetMaxSpeed (Variables|Default|GetFloatingPawnMovement) _output_get))

(fn ConstructionScript)