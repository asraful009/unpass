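; FloorBP is a self-chaining floor segment for what appears to be an endless runner.
; PlayerPawnBP overlaps spawn the next segment at the Arrow, destroy this one on leaving DeleteThisFloor, and call OnDead on leaving RestGame.
; A looping timer spawns ObostracleBP using a random point in Obs01's box; Obs02–04 are unused.
; ObsSpawnPosition prints debug text and adds the box's world location twice, offsetting spawns.
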(event OnComponentBeginOverlap(CreateNextFloor)
  (params (OverlappedComponent :type Primitive%20Component%20Object%20Reference) (OtherActor :type Actor%20Object%20Reference) (OtherComp :type Primitive%20Component%20Object%20Reference) (OtherBodyIndex :type Integer) (bFromSweep :type Boolean) (SweepResult :type Hit%20Result%20Structure%20%28by%20ref%29))
  (bind _arrow (Variables|Default|GetArrow))
  (bind _returnvalue (Transformation|GetWorldTransform _arrow))
  (Utilities|Casting|CastToPlayerPawnBP OtherActor)
  (Game|SpawnActorfromClass "FloorBP_C" (Math|Transform|MakeTransform (.location _returnvalue) (.rotation _returnvalue)) "Undefined" 0 0))

(event OnComponentEndOverlap(DeleteThisFloor)
  (params (OverlappedComponent :type Primitive%20Component%20Object%20Reference) (OtherActor :type Actor%20Object%20Reference) (OtherComp :type Primitive%20Component%20Object%20Reference) (OtherBodyIndex :type Integer))
  (Utilities|Casting|CastToPlayerPawnBP OtherActor)
  (Actor|DestroyActor))

(event OnComponentEndOverlap(RestGame)
  (params (OverlappedComponent :type Primitive%20Component%20Object%20Reference) (OtherActor :type Actor%20Object%20Reference) (OtherComp :type Primitive%20Component%20Object%20Reference) (OtherBodyIndex :type Integer))
  (bind _asplayer_pawn_bp (Utilities|Casting|CastToPlayerPawnBP OtherActor))
  (Default|OnDead _asplayer_pawn_bp))

(event Custom|MyE
  (Game|SpawnActorfromClass "/Game/blueprint/ObostracleBP.ObostracleBP_C" (Math|Transform|MakeTransform (CallFunction|ObsSpawnPosition (Variables|Default|GetObs-01))) "Undefined" 0 0))

(event EventBeginPlay
  (Utilities|Time|SetTimerbyEvent (delegate Custom|MyE) 2.0 true))

(event Collision|EventActorBeginOverlap
  (params (OtherActor :type Actor%20Object%20Reference)))

(event EventTick
  (params (DeltaSeconds :type Float%20%28single-precision%29)))

(fn ConstructionScript)

(fn ObsSpawnPosition
  (params (ObsObj :type Box%20Component%20Object%20Reference))
  (bind _returnvalue (Transformation|GetWorldLocation ObsObj))
  (bind _boxextent (Variables|/Script/Engine.BoxComponent|GetBoxExtent ObsObj))
  (bind _returnvalue_2 (Math|Random|RandomPointinBoundingBox _returnvalue _boxextent))
  (bind _returnvalue_3 (+ _returnvalue _returnvalue_2))
  (Development|PrintString (Utilities|String|Append (Utilities|String|ToString(Vector) _returnvalue) "++++" (Utilities|String|ToString(Vector) _returnvalue) "+" (Utilities|String|ToString(Vector) _boxextent) "=" (Utilities|String|ToString(Vector) _returnvalue_3)) true true "(R=0.000000,G=0.660000,B=1.000000,A=1.000000)" 1e+01)
  (return _returnvalue_3))