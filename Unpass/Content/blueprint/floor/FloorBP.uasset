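; FloorBP is a floor segment that builds an endlessly extending track for Car4BP, with randomly placed obstacles.
; On BeginPlay, it hides its placement boxes and spawns one obstacle in each, at a random point and yaw.
; When the car overlaps CreateNextFloor, a random floor class spawns at the Arrow's transform.
; Overlapping DeleteThisFloor calls DestoryEvent on the tracked obstacles, then destroys the segment.
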(event OnComponentBeginOverlap(CreateNextFloor)
  (params (OverlappedComponent :type Primitive%20Component%20Object%20Reference) (OtherActor :type Actor%20Object%20Reference) (OtherComp :type Primitive%20Component%20Object%20Reference) (OtherBodyIndex :type Integer) (bFromSweep :type Boolean) (SweepResult :type Hit%20Result%20Structure%20%28by%20ref%29))
  (bind _arrow (Variables|Default|GetArrow))
  (bind _returnvalue (Transformation|GetWorldTransform _arrow))
  (Utilities|Casting|CastToCar4BP OtherActor)
  (bind _returnvalue_2 (Game|SpawnActorfromClass (.OutItem (Utilities|Array|Random (Variables|Default|Getfloor))) (Math|Transform|MakeTransform (.location _returnvalue) (.rotation _returnvalue)) "Undefined" 0 0))
  (Development|PrintString (Utilities|GetDisplayName _returnvalue_2)))

(event OnComponentBeginOverlap(DeleteThisFloor)
  (params (OverlappedComponent :type Primitive%20Component%20Object%20Reference) (OtherActor :type Actor%20Object%20Reference) (OtherComp :type Primitive%20Component%20Object%20Reference) (OtherBodyIndex :type Integer) (bFromSweep :type Boolean) (SweepResult :type Hit%20Result%20Structure%20%28by%20ref%29))
  (Utilities|Casting|CastToCar4BP OtherActor)
  (for _array_element (Variables|Obj|GetallObs)
    (Default|DestoryEvent _array_element))
  (Actor|DestroyActor))

(event EventBeginPlay
  (CallFunction|CreateObsbyPosition))

(event Collision|EventActorBeginOverlap
  (params (OtherActor :type Actor%20Object%20Reference)))

(fn ConstructionScript)

(fn ObsSpawnPosition
  (params (ObsObj :type Box%20Component%20Object%20Reference))
  (bind _returnvalue (Transformation|GetWorldRotation ObsObj))
  (return (Math|Random|RandomPointinBoundingBox (Transformation|GetWorldLocation ObsObj) (Variables|/Script/Engine.BoxComponent|GetBoxExtent ObsObj)) (Math|Rotator|MakeRotator (.roll _returnvalue) (.pitch _returnvalue) (.yaw (Math|Random|RandomRotator false)))))

(fn CreateObj
  (params (ObsObj :type Box%20Component%20Object%20Reference))
  (bind (_position _rotation) (CallFunction|ObsSpawnPosition ObsObj))
  (bind _returnvalue (Game|SpawnActorfromClass "/Game/blueprint/obs/Obs-01.Obs-01_C" (Math|Transform|MakeTransform _position _rotation) "Undefined" 0 0))
  (Utilities|Array|Add (Variables|Obj|GetallObs) _returnvalue))

(fn CreateObsbyPosition
  (Variables|obj|SetsPososion (Utilities|Array|MakeArray (Variables|ObsPosition|GetObs-017) (Variables|ObsPosition|GetObs-019) (Variables|ObsPosition|GetObs-025) (Variables|ObsPosition|GetObs-027) (Variables|ObsPosition|GetObs-016) (Variables|ObsPosition|GetObs-01) (Variables|ObsPosition|GetObs-03) (Variables|ObsPosition|GetObs-04)))
  (for _array_element (Variables|obj|GetsPososion)
    (Development|SetHiddeninGame _array_element true false)
    (CallFunction|CreateObj _array_element)))