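; Car4BP is a drivable car Blueprint with an orbitable spring arm camera.
; Move axes feed throttle and steering on the vehicle movement component, and mouse axes add relative yaw and pitch to the spring arm.
; Each tick passes engine rotation speed to the engine sound's RPM parameter.
; GetWheelPlayerRef prints the car's display name and returns the car itself.
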(event EventBeginPlay)

(event Collision|EventActorBeginOverlap
  (params (OtherActor :type Actor%20Object%20Reference)))

(event EventTick
  (params (DeltaSeconds :type Float%20%28single-precision%29))
  (Audio|Parameter|SetFloatParameter (Variables|Default|GetEngineSound) "RPM" (Class|WheeledVehicleMovementComponent|GetEngineRotationSpeed (Variables|Default|GetVehicleMovement)) :!class /Script/Engine.AudioComponent))

(event Input|AxisEvents|InputAxisMoveFwd
  (params (AxisValue :type Float%20%28single-precision%29))
  (Class|WheeledVehicleMovementComponent|SetThrottleInput (Variables|Default|GetVehicleMovement) AxisValue))

(event Input|AxisEvents|InputAxisMoveLeftRight
  (params (AxisValue :type Float%20%28single-precision%29))
  (Class|WheeledVehicleMovementComponent|SetSteeringInput (Variables|Default|GetVehicleMovement) AxisValue))

(event Input|MouseEvents|MouseX
  (params (AxisValue :type Float%20%28single-precision%29))
  (Transformation|AddRelativeRotation (Variables|Default|GetSpringArm) (Math|Rotator|MakeRotator 0.0 0.0 AxisValue) false false))

(event Input|MouseEvents|MouseY
  (params (AxisValue :type Float%20%28single-precision%29))
  (Transformation|AddRelativeRotation (Variables|Default|GetSpringArm) (Math|Rotator|MakeRotator 0.0 AxisValue 0.0) false false))

(fn ConstructionScript)

(fn GetWheelPlayerRef
  (bind _self self)
  (Development|PrintString (Utilities|GetDisplayName _self))
  (return _self))